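; BP_Ball is a ball actor that bounces off whatever it hits, moving only in the YZ plane after each bounce.
; Tick moves it by Velocity times Speed with a swept SetActorLocation, so collisions fire Hit.
; Hit raises Speed by a fixed step up to a cap, mirrors Velocity by the hit normal, then zeroes X and normalizes to prevent stray directions.
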(event `self.ReceiveTick`
  (params (DeltaSeconds :type "Float (single-precision)"))
  (`self.K2_SetActorLocation` (+ (`self.K2_GetActorLocation`) (* (* (`self.Velocity`) (`self.Speed`)) DeltaSeconds)) true))

(event `self.ReceiveHit`
  (params (MyComp :type "PrimitiveComponent Object Reference") (Other :type "Actor Object Reference") (OtherComp :type "PrimitiveComponent Object Reference") (bSelfMoved :type Boolean) (HitLocation :type "Vector Structure") (HitNormal :type "Vector Structure") (NormalImpulse :type "Vector Structure") (Hit :type "HitResult Structure (by ref)"))
  (set `self.Speed` (`KismetMathLibrary.FMin` (+ (`self.Speed`) 50.0) 500.0)) ; 壁に当たったときはスピードを更新
  (set `self.Velocity` (`KismetMathLibrary.Normal` (`KismetMathLibrary.MakeVector` 0.0 (.y (`KismetMathLibrary.MirrorVectorByNormal` (`self.Velocity`) HitNormal)) (.z (`KismetMathLibrary.MirrorVectorByNormal` (`self.Velocity`) HitNormal))))))

(fn `UserConstructionScript`)