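; Game mode for a block-breaker game that sets up the session and handles block breaks, lost balls and game over.
; BeginPlay sets a portrait window, shows the cursor, adds joypad and score widgets, and resets balls and score through GameState messages.
; Block breaks add score and check for stage clear, whose handler is empty.
; Lost balls check remaining balls before notifying GameState, then restart or trigger game over, which disables input and swaps widgets.
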(event `self.ReceiveBeginPlay`
  (`|ExecutionSequence`
    (:`then_0`
      (`self.InitEnv`))
    (:`then_1`
      (`self.InitGame`))))

(event `/Game/Blueprints/Main/IF_GameEvent.BreakBlock`
  (params (addScore :type Integer))
  (message `/Game/Blueprints/Main/IF_MyGameState.AddScore` (`GameplayStatics.GetGameState`) addScore)
  (bind _stageclear (`self.IsStageClear?`))
  (if _stageclear
    (message `/Game/Blueprints/Main/IF_GameEvent.StageClear` (`GameplayStatics.GetGameMode`))))

(event `/Game/Blueprints/Main/IF_GameEvent.LostBall`
  (bind _returnvalue (`GameplayStatics.GetGameMode`))
  (`|ExecutionSequence`
    (:`then_0`
      (bind _gameover (`self.IsGameOver?`))
      (if _gameover
        (message `/Game/Blueprints/Main/IF_GameEvent.GameOver` _returnvalue)
        (else
          (message `/Game/Blueprints/Main/IF_GameEvent.RestartBall` _returnvalue))))
    (:`then_1`
      (message `/Game/Blueprints/Main/IF_MyGameState.LostBall` (`GameplayStatics.GetGameState`)))))

(event `/Game/Blueprints/Main/IF_GameEvent.StageClear`)

(event `/Game/Blueprints/Main/IF_GameEvent.GameOver`
  (`|ExecutionSequence`
    (:`then_0`
      (`self.DisableInput` (`GameplayStatics.GetPlayerController` 0)))
    (:`then_1`
      (`WidgetLayoutLibrary.RemoveAllWidgets`))
    (:`then_2`
      (bind _returnvalue (`|CreateWidget` "/Game/UI/Main/UI_Gameover.UI_Gameover_C"))
      (`UserWidget.AddToViewport` _returnvalue 0))))

(fn `InitEnv`
  (`|ExecutionSequence`
    (:`then_0`
      (bind _returnvalue (`GameUserSettings.GetGameUserSettings`))
      (`GameUserSettings.SetScreenResolution` _returnvalue (make `IntPoint` 800 1280)) ; ウィンドウサイズの設定を行う
      (`GameUserSettings.ApplySettings` _returnvalue true))
    (:`then_1`
      (set `PlayerController.bShowMouseCursor` true (`GameplayStatics.GetPlayerController` 0)))
    (:`then_2`
      (`|ExecutionSequence`
        (:`then_0`
          (bind _asbp_my_player_controller (cast `/Game/Blueprints/Main/BP_MyPlayerController` (`GameplayStatics.GetPlayerController` 0)))
          (bind _returnvalue_2 (`|CreateWidget` "/Game/UI/Main/UI_Joypad.UI_Joypad_C" null _asbp_my_player_controller))
          (`UserWidget.AddToViewport` _returnvalue_2 0))
        (:`then_1`
          (bind _returnvalue_3 (`|CreateWidget` "/Game/UI/Main/UI_Score.UI_Score_C"))
          (`UserWidget.AddToViewport` _returnvalue_3 0))))))

(fn `InitGame`
  (`|ExecutionSequence`
    (:`then_0`
      (message `/Game/Blueprints/Main/IF_MyGameState.ResetBalls` (`GameplayStatics.GetGameState`)))
    (:`then_1`
      (message `/Game/Blueprints/Main/IF_MyGameState.ResetScore` (`GameplayStatics.GetGameState`)))))

(fn `IsGameOver?`
  (returns (gameover :type Boolean))
  (bind _balls (message `/Game/Blueprints/Main/IF_MyGameState.GetBalls` (`GameplayStatics.GetGameState`)))
  (return (<= _balls 0)))

(fn `IsStageClear?`
  (returns (stageClear :type Boolean))
  (bind _blockcount (message `/Game/Blueprints/Main/IF_MyGameState.GetBlockCount` (`GameplayStatics.GetGameState`)))
  (return (<= _blockcount 0)))

(fn `UserConstructionScript`)