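; BP_MyGameMode is the game mode for a block-breaking ball game, handling setup, scoring, lost balls and game over.
; On BeginPlay it shows the mouse cursor and resets balls and score through message calls to the GameState.
; BreakBlock forwards score to the GameState.
; LostBall checks remaining balls to trigger game over or ball restart, then notifies the GameState afterwards; GameOver only prints debug text.
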(event `self.ReceiveBeginPlay`
  (`|ExecutionSequence`
    (:`then_0`
      (`self.InitEnv`))
    (:`then_1`
      (`self.InitGame`))))

(event `/Game/Blueprints/IF_GameEvent.BreakBlock`
  (params (addScore :type Integer))
  (message `/Game/Blueprints/IF_MyGameState.AddScore` (`GameplayStatics.GetGameState`) addScore))

(event `/Game/Blueprints/IF_GameEvent.LostBall`
  (bind _returnvalue (`GameplayStatics.GetGameMode`))
  (`|ExecutionSequence`
    (:`then_0`
      (bind _gameover (`self.IsGameOver?`))
      (if _gameover
        (message `/Game/Blueprints/IF_GameEvent.GameOver` _returnvalue)
        (else
          (message `/Game/Blueprints/IF_GameEvent.RestartBall` _returnvalue))))
    (:`then_1`
      (message `/Game/Blueprints/IF_MyGameState.LostBall` (`GameplayStatics.GetGameState`)))))

(event `/Game/Blueprints/IF_GameEvent.GameOver`
  (`KismetSystemLibrary.PrintString` "game over!!!!!!!!!!!!!!!!!!!!!!!!!!!!!!!!!!!!"))

(fn `InitEnv`
  (set `PlayerController.bShowMouseCursor` true (`GameplayStatics.GetPlayerController` 0)))

(fn `InitGame`
  (`|ExecutionSequence`
    (:`then_0`
      (message `/Game/Blueprints/IF_MyGameState.ResetBalls` (`GameplayStatics.GetGameState`)))
    (:`then_1`
      (message `/Game/Blueprints/IF_MyGameState.ResetScore` (`GameplayStatics.GetGameState`)))))

(fn `IsGameOver?`
  (returns (gameover :type Boolean))
  (bind _balls (message `/Game/Blueprints/IF_MyGameState.GetBalls` (`GameplayStatics.GetGameState`)))
  (return (<= _balls 0)))

(fn `UserConstructionScript`)