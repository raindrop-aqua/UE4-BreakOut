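; BP_MyGameState is a game state that tracks score, remaining balls and block count for what appears to be a block-breaker game.
; Events count blocks as they are added, add points while decrementing the block count, and decrement balls when one is lost, guarded against going below zero.
; Reset events restore the starting ball count and zero the score, and simple getters expose all three values.
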(event `/Game/Blueprints/IF_MyGameState.AddBlock`
  (bind _result (`/Engine/EditorBlueprintResources/StandardMacros.IncrementInt` (`self.BlockCount`))
    (:`  `
      (set `self.BlockCount` _result) ; ブロック数加算
    )))

(event `/Game/Blueprints/IF_MyGameState.AddScore`
  (params (score :type Integer))
  (`|ExecutionSequence`
    (:`then_0`
      (set `self.Score` (+ (`self.Score`) score)) ; スコア加算
    )
    (:`then_1`
      (bind _result (`/Engine/EditorBlueprintResources/StandardMacros.DecrementInt` (`self.BlockCount`))
        (:`  `
          (set `self.BlockCount` _result) ; ブロック数減算
        )))))

(event `/Game/Blueprints/IF_MyGameState.LostBall`
  (if (> (`self.Balls`) 0)
    (bind _result (`/Engine/EditorBlueprintResources/StandardMacros.DecrementInt` (`self.Balls`))
      (:`  `
        (set `self.Balls` _result)))))

(event `/Game/Blueprints/IF_MyGameState.ResetBalls`
  (set `self.Balls` 3) ; 初期数に設定する
)

(event `/Game/Blueprints/IF_MyGameState.ResetScore`
  (set `self.Score` 0) ; ゼロに設定する
)

(fn `GetBalls`
  (returns (balls :type Integer))
  (return (`self.Balls`)))

(fn `GetBlockCount`
  (returns (blockCount :type Integer))
  (return (`self.BlockCount`)))

(fn `GetScore`
  (returns (score :type Integer))
  (return (`self.Score`)))

(fn `UserConstructionScript`)